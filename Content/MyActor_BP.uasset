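; Actor that visualizes an AngularVelocity vector with a scaled and oriented cylinder and mesh.
; Each tick it stretches and offsets Cylinder along local down by the vector's magnitude.
; VisualMesh aligns down to the vector via a 180-degree turn around their bisector, with a fallback for the degenerate case.
; BeginPlay enables player input, and key 1 sets a Canstart flag that nothing in these graphs reads.
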(event EventBeginPlay
  ;[1 1 1] get input
  (Input|EnableInput (Game|GetPlayerController 0)))

(event EventTick
  (params (DeltaSeconds :type Float%20%28single-precision%29))
  (bind _returnvalue (Math|Vector|VectorDown))
  (bind _angularvelocity (Variables|Default|GetangularVelocity))
  (bind _returnvalue_2 (Math|Vector|VectorLength _angularvelocity))
  (bind _returnvalue_3 (Math|Vector|GetUnitDirection(Vector) "0, 0, 0" _angularvelocity))
  (bind _returnvalue_4 (/ _returnvalue_2 1e+01))
  (bind _returnvalue_5 (+ _returnvalue_3 _returnvalue))
  (Transformation|SetRelativeScale3D (Variables|Default|GetCylinder) (Math|Vector|MakeVector 0.5 0.5 _returnvalue_4))
  (Transformation|SetRelativeLocation (Variables|Default|GetCylinder) (* _returnvalue (* _returnvalue_4 5e+01)) false false)
  (if (Math|Vector|VectorIsNearlyZero _returnvalue_5)
    (Transformation|SetWorldRotation (Variables|Default|GetVisualMesh) "180.000000,0.000000, 0" false false)
    (else
      (Transformation|SetWorldRotation (Variables|Default|GetVisualMesh) (Math|Vector|RotatorfromAxisandAngle _returnvalue_5 1.8e+02) false false))))

(event Input|KeyboardEvents|1
  (params (Key :type Key%20Structure :default "None"))
  (:Pressed
    (Variables|Default|Setcanstart true)))

(fn ConstructionScript)